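; Player character Blueprint for the Unseen GAS character, adding a pause menu toggle on top of its parent class.
; The IA_PauseGame Enhanced Input action flips IsPauseMenuOpened, showing or hiding PauseMenuWidget and pausing or resuming the game.
; Each toggle also switches between Game-and-UI and Game-only input modes and shows or hides the mouse cursor.
; BeginPlay, Tick, overlap and the construction script are empty.
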(event `self.ReceiveBeginPlay`)

(event `EnhancedInput|/Game/ThirdPerson/Input/Actions/IA_PauseGame`
  (params (ActionValue :type Boolean) (ElapsedSeconds :type "Float (double-precision)") (TriggeredSeconds :type "Float (double-precision)") (InputAction :type "InputAction Object Reference" :default "/Game/ThirdPerson/Input/Actions/IA_PauseGame.IA_PauseGame"))
  (bind _returnvalue (`GameplayStatics.GetPlayerController` 0))
  (:`Started`
    (if (not (`self.IsPauseMenuOpened`))
      (set `self.IsPauseMenuOpened` true)
      (`Widget.SetVisibility` (`self.PauseMenuWidget`) "Visible")
      (`WidgetBlueprintLibrary.SetInputMode_GameAndUIEx` _returnvalue (`self.PauseMenuWidget`))
      (set `PlayerController.bShowMouseCursor` true (`GameplayStatics.GetPlayerController` 0))
      (`GameplayStatics.SetGamePaused` true)
      (else
        (set `self.IsPauseMenuOpened` false)
        (`Widget.SetVisibility` (`self.PauseMenuWidget`) "Hidden")
        (`GameplayStatics.SetGamePaused` false)
        (`WidgetBlueprintLibrary.SetInputMode_GameOnly` _returnvalue)
        (set `PlayerController.bShowMouseCursor` false (`GameplayStatics.GetPlayerController` 0))))))

(fn `UserConstructionScript`)