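; Earth boss Blueprint that provides three montage-driven combat actions: attack, teleport and an area skill.
; Each action sets a busy flag while its montage plays, blocking re-triggering of that same action.
; Skill1 calls SetSkillPos, then spawns a short-lived SkillPosCheck actor and moves the Niagara effect there.
; A montage notify fires the explosion sound and VFX, which are hidden shortly after the montage completes.
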(event `/Game/Boss/BPI_BossFight.Attack`
  ;[1 1 1] Attack
  (if (not (`self.isAttacking?`))
    (`|PlayMontage` (`self.Mesh`) "/Game/Boss/AM_Attack.AM_Attack"
      (:`then`
        (set `self.isAttacking?` true))
      (:`OnCompleted`
        (set `self.isAttacking?` false)))))

(event `/Game/Boss/BPI_BossFight.Teleport`
  (if (not (`self.isTeleporting?`))
    (`|PlayMontage` (`self.Mesh`) "/Game/Boss/AM_Teleport.AM_Teleport"
      (:`then`
        (set `self.isTeleporting?` true))
      (:`OnCompleted`
        (set `self.isTeleporting?` false)))))

(event `/Game/Boss/BPI_BossFight.Skill1`
  (bind _skillniagara (`self.SkillNiagara`))
  (bind _skillniagara_2 (`self.SkillNiagara`))
  (if (not (`self.isSkill1`))
    (`self.SetSkillPos`)
    (bind _returnvalue (`|SpawnActorFromClass` "/Game/Boss/SkillPosCheck.SkillPosCheck_C" (`KismetMathLibrary.MakeTransform` (`self.SkillPos`) (struct) (10.3 10.3 1.0)) "Undefined" "MultiplyWithRoot" null null))
    (`self.SetLifeSpan` _returnvalue 0.5)
    (`SceneComponent.K2_SetWorldLocation` (`self.SkillNiagara`) (`self.SkillPos`) false true)
    (`|PlayMontage` (`self.Mesh`) "/Game/Boss/AM_Skill_01.AM_Skill_01"
      (:`then`
        (set `self.isSkill1` true))
      (:`OnCompleted`
        (`KismetSystemLibrary.Delay` 1.5)
        (`ActorComponent.Deactivate` _skillniagara)
        (`SceneComponent.SetHiddenInGame` _skillniagara true false)
        (set `self.isSkill1` false))
      (:`OnNotifyBegin`
        (`GameplayStatics.PlaySound2D` "/Game/Sound/explosion_Cue.explosion_Cue" 1.0 1.0 0.0 null null)
        (`ActorComponent.Activate` _skillniagara_2 true)
        (`ActorComponent.Activate` (`self.SkillNiagara`) true)
        (`SceneComponent.SetHiddenInGame` _skillniagara_2 false false)))))

(fn `UserConstructionScript`)